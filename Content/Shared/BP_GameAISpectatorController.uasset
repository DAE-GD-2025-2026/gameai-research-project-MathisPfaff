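; Controller for the GameAI spectator that turns Enhanced Input actions into camera movement and look.
; Separate 2D (locked) and free move actions both feed movement input to the controlled pawn, converted from the GameAISpectator root's local space to world space.
; Mouse look adds yaw and inverted pitch input to the controlled pawn.
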(event `EnhancedInput|/Game/Input/IA_Move2D`
  (params (ActionValue :type "Vector Structure") (ElapsedSeconds :type "Float (double-precision)") (TriggeredSeconds :type "Float (double-precision)") (InputAction :type "InputAction Object Reference" :default "/Game/Input/IA_Move2D.IA_Move2D"))
  ; Locked Spectator Movement
  (:`Triggered`
    (`Pawn.AddMovementInput` (`Controller.K2_GetPawn`) (`KismetMathLibrary.TransformDirection` (`SceneComponent.K2_GetComponentToWorld` (`Actor.RootComponent` (`self.GameAISpectator`))) ActionValue) 1.0 false)))

(event `EnhancedInput|/Game/Input/IA_Move`
  (params (ActionValue :type "Vector Structure") (ElapsedSeconds :type "Float (double-precision)") (TriggeredSeconds :type "Float (double-precision)") (InputAction :type "InputAction Object Reference" :default "/Game/Input/IA_Move.IA_Move"))
  ; Free Spectator Movement
  (:`Triggered`
    (`Pawn.AddMovementInput` (`Controller.K2_GetPawn`) (`KismetMathLibrary.TransformDirection` (`SceneComponent.K2_GetComponentToWorld` (`Actor.RootComponent` (`self.GameAISpectator`))) ActionValue) 1.0 false)))

(event `EnhancedInput|/Game/Input/IA_MouseLook`
  (params (ActionValue :type "Vector2D Structure") (ElapsedSeconds :type "Float (double-precision)") (TriggeredSeconds :type "Float (double-precision)") (InputAction :type "InputAction Object Reference" :default "/Game/Input/IA_MouseLook.IA_MouseLook"))
  ; Free Spectator Movement
  (:`Triggered`
    (`|ExecutionSequence`
      (:`then_0`
        (`Pawn.AddControllerYawInput` (`Controller.K2_GetPawn`) ActionValue_X))
      (:`then_1`
        (`Pawn.AddControllerPitchInput` (`Controller.K2_GetPawn`) (* ActionValue_Y -1.0))))))

(fn `UserConstructionScript`)